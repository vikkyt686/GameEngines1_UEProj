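; Water hazard that damages the third-person character on entering its trigger while a linked power box is on.
; It binds to the power box's power event at BeginPlay and uses its state to set the damage amount and toggle sparks and audio.
; Damage applies once per trigger overlap, replaying the audio and activating sparks.
; Audio also starts at BeginPlay without checking the power state.
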(event `self.ReceiveBeginPlay`
  (`parent.ReceiveBeginPlay`)
  (add `/Game/MyBlueprints/BP_PowerBox.PowerOn` (`self.PowerBoxRef`) (delegate `UpdateWaterState`))
  (`AudioComponent.Play` (`self.Audio`) (`self.StartTimeOffset`)))

(event `self.ReceiveActorBeginOverlap`
  (params (OtherActor :type "Actor Object Reference"))
  (`parent.ReceiveActorBeginOverlap` OtherActor))

(event `UpdateWaterState`
  (`self.UpdateWaterElectrifiedState` (`/Game/MyBlueprints/BP_PowerBox.bIsPowerOn` (`self.PowerBoxRef`))))

(event `self.DamageTrigger.OnComponentBeginOverlap`
  (params (OverlappedComponent :type "PrimitiveComponent Object Reference") (OtherActor :type "Actor Object Reference") (OtherComp :type "PrimitiveComponent Object Reference") (OtherBodyIndex :type Integer) (bFromSweep :type Boolean) (SweepResult :type "HitResult Structure (by ref)"))
  (bind _asbp_third_person_character (cast `/Game/ThirdPerson/Blueprints/BP_ThirdPersonCharacter` OtherActor))
  (if (`/Game/MyBlueprints/BP_PowerBox.bIsPowerOn` (`self.PowerBoxRef`))
    (`GameplayStatics.ApplyDamage` _asbp_third_person_character (`self.Damage Amount`))
    (`AudioComponent.Play` (`self.Audio`) 0.0)
    (`ActorComponent.SetActive` (`self.Sparks1`) true false)))

(fn `UpdateWaterElectrifiedState`
  (params (Active :type Boolean))
  (bind _audio (`self.Audio`))
  (bind _sparks1 (`self.Sparks1`))
  (if Active
    (set `self.Damage Amount` 100.0)
    (`ActorComponent.SetActive` _sparks1 Active false)
    (`SceneComponent.SetVisibility` _sparks1 Active false)
    (`AudioComponent.Play` _audio (`self.StartTimeOffset`))
    (else
      (set `self.Damage Amount` 0.0)
      (`ActorComponent.SetActive` _sparks1 Active false)
      (`SceneComponent.SetVisibility` _sparks1 Active false)
      (`AudioComponent.Stop` _audio))))

(fn `UserConstructionScript`
  (`parent.UserConstructionScript`))