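; BP_Tickets animates a stack of tickets being printed out by scrolling its material.
; On BeginPlay it creates a dynamic instance of MI_TicketStack on the TicketStack component.
; The SpitOutTickets event plays a timeline that drives the material's UOffset parameter, so the motion comes from the material.
; DonePrinting is cleared at the start and set when the timeline finishes, alongside a debug print.
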(event `self.ReceiveBeginPlay`
  (bind _returnvalue (`PrimitiveComponent.CreateDynamicMaterialInstance` (`self.TicketStack`) 0 "/Game/MyMaterials/MI_TicketStack.MI_TicketStack" "None"))
  (set `self.DMI_Mat_TicketStack` _returnvalue))

(event `SpitOutTickets`
  (set `self.bDonePrinting` false)
  (bind (_direction _uoffset) (`Timeline|SpittingTickets` :!via `PlayFromStart`)
    (:`Update`
      (`MaterialInstanceDynamic.SetScalarParameterValue` (`self.DMI_Mat_TicketStack`) "UOffset" _uoffset))
    (:`Finished`
      (`KismetSystemLibrary.PrintString` "Done printing tickets!" true true (struct :`R` 0.007687 :`G` 1.0 :`A` 1.0) 3.0)
      (set `self.bDonePrinting` true))))

(fn `UserConstructionScript`)