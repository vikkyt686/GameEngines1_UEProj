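; Front door actor whose metal door gives way to physics once the back door has been unlocked.
; When the third-person character overlaps the interactible area, it checks the referenced back door's unlocked flag, then enables physics on the door and updates the character's objective.
; An actor-hit event bound at BeginPlay plays a thud at the actor's location whenever a hit occurs while the door is simulating physics.
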(event `self.InteractibleArea.OnComponentBeginOverlap`
  (params (OverlappedComponent :type "PrimitiveComponent Object Reference") (OtherActor :type "Actor Object Reference") (OtherComp :type "PrimitiveComponent Object Reference") (OtherBodyIndex :type Integer) (bFromSweep :type Boolean) (SweepResult :type "HitResult Structure (by ref)"))
  (bind _asbp_third_person_character (cast `/Game/ThirdPerson/Blueprints/BP_ThirdPersonCharacter` OtherActor))
  (if (`/Game/MyBlueprints/BP_LockedDoor.bBackDoorUnlocked` (`self.BP_BackDoorRef`))
    (`PrimitiveComponent.SetSimulatePhysics` (`self.MetalDoor`) true)
    (`/Game/ThirdPerson/Blueprints/BP_ThirdPersonCharacter.UpdateObjective` _asbp_third_person_character "NewEnumerator7")))

(event `self.ReceiveBeginPlay`
  (add `self.OnActorHit` (delegate `OnActorHit_Event`)))

(event `OnActorHit_Event` :!signature `self.OnActorHit`
  (params (SelfActor :type "Actor Object Reference") (OtherActor :type "Actor Object Reference") (NormalImpulse :type "Vector Structure") (Hit :type "HitResult Structure (by ref)"))
  (if (`SceneComponent.IsSimulatingPhysics` (`self.MetalDoor`) "None")
    (`GameplayStatics.PlaySoundAtLocation` "/Game/MyAudio/thud.thud" (`self.K2_GetActorLocation`) (struct) 1.0 1.0 0.0 null null null null)))

(fn `UserConstructionScript`)