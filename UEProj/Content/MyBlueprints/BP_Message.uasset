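; BP_Message is a trigger actor that gives the player a new objective when BP_ThirdPersonCharacter overlaps its MessageTrigger.
; It passes CurrObjective to the character's UpdateObjective and, on success, animates the new objective on the cached player's HUD.
; If DestroyOnceRead is set, it then flags itself against re-triggering and destroys itself after a short delay.
; A SetAndDisplayMessage function for timed text and sound remains, but its call is disconnected.
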(event `self.ReceiveBeginPlay`
  (bind _asbp_third_person_character (cast `/Game/ThirdPerson/Blueprints/BP_ThirdPersonCharacter` (`GameplayStatics.GetPlayerCharacter` 0)))
  (set `self.The Player` _asbp_third_person_character))

(event `self.MessageTrigger.OnComponentBeginOverlap`
  (params (OverlappedComponent :type "PrimitiveComponent Object Reference") (OtherActor :type "Actor Object Reference") (OtherComp :type "PrimitiveComponent Object Reference") (OtherBodyIndex :type Integer) (bFromSweep :type Boolean) (SweepResult :type "HitResult Structure (by ref)"))
  (if (not (`self.bPendingDestroy`))
    (bind _asbp_third_person_character (cast `/Game/ThirdPerson/Blueprints/BP_ThirdPersonCharacter` OtherActor))
    (bind _bupdatedobjective (`/Game/ThirdPerson/Blueprints/BP_ThirdPersonCharacter.UpdateObjective` _asbp_third_person_character (`self.CurrObjective`)))
    (if _bupdatedobjective
      (`/Game/InterfaceWidgets/HUDWidget.AnimateNewObjective` (`/Game/ThirdPerson/Blueprints/BP_ThirdPersonCharacter.My HUD` (`self.The Player`)))
      (if (`self.bDestroyOnceRead`)
        (set `self.bPendingDestroy` true)
        (`KismetSystemLibrary.Delay` 3.0)
        (`self.K2_DestroyActor`)))))

(fn `Set and Display Message`
  (bind _bdisplayed (`self.bDisplayed`))
  (if (`self.bDisplayOnce`)
    (if (not _bdisplayed)
      (`/Game/ThirdPerson/Blueprints/BP_ThirdPersonCharacter.DisplayMessage` (`self.The Player`) (`self.MyMessage`) (`self.Display Time`) :!label _label)
      (`GameplayStatics.PlaySoundAtLocation` "/Game/MyAudio/Rollover.Rollover" (`self.K2_GetActorLocation`) (struct) 1.0 1.0 0.0 null null null null :!label _label_2)
      (set `self.bDisplayed` true))
    (elif _bdisplayed
      (goto _label_2)
      (else
        (goto _label)))))

(fn `UserConstructionScript`)