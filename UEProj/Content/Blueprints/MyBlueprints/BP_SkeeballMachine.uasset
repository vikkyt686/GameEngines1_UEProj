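; Skeeball minigame machine, playable while its power box is on, that awards collectible tickets advancing the player's objective.
; Successive interact presses lock looping-timer sweeps of aim and power, then launch the physics ball by impulse.
; Trigger zones add points and reset the ball.
; The roll-down trigger or reset input also checks game over, spawning BP_Tickets once balls exceed the limit with at least 300 points.
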(event `self.ReceiveBeginPlay`
  ;[0 0 0] Begin Play
  (bind _asbp_third_person_character (cast `/Game/ThirdPerson/Blueprints/BP_ThirdPersonCharacter` (`GameplayStatics.GetPlayerCharacter` 0)))
  (set `self.PlayerRef` _asbp_third_person_character)
  (`self.EnableInput` (`GameplayStatics.GetPlayerController` 0))
  (set `self.BallStartTransform` (`SceneComponent.K2_GetComponentToWorld` (`self.Ball`)))
  (`SceneComponent.SetVisibility` (`self.ScoreText`) false false)
  (`SceneComponent.SetVisibility` (`self.Arrow`) false false)
  (`SceneComponent.SetVisibility` (`self.Ball`) false false))

(event `self.InteractArea.OnComponentBeginOverlap`
  (params (OverlappedComponent :type "PrimitiveComponent Object Reference") (OtherActor :type "Actor Object Reference") (OtherComp :type "PrimitiveComponent Object Reference") (OtherBodyIndex :type Integer) (bFromSweep :type Boolean) (SweepResult :type "HitResult Structure (by ref)"))
  (cast `/Game/ThirdPerson/Blueprints/BP_ThirdPersonCharacter` OtherActor)
  (if (`/Game/Blueprints/MyBlueprints/BP_ElectricalBox.bIsPowerOn` (`self.BP_PowerBox`))
    (if (`self.bIsCompleted`)
      (`self.ClearTimers`) ; only as a precaution - shouldn't really be needed
      (else
        (`SceneComponent.SetVisibility` (`self.InteractText`) true false)))))

(event `self.InteractArea.OnComponentEndOverlap`
  (params (OverlappedComponent :type "PrimitiveComponent Object Reference") (OtherActor :type "Actor Object Reference") (OtherComp :type "PrimitiveComponent Object Reference") (OtherBodyIndex :type Integer))
  (cast `/Game/ThirdPerson/Blueprints/BP_ThirdPersonCharacter` OtherActor)
  (`SceneComponent.SetVisibility` (`self.InteractText`) false false)
  (`SceneComponent.SetVisibility` (`self.Widget_SkeeballPower`) false false)
  (`SceneComponent.SetVisibility` (`self.Widget_HorizontalPosition`) false false))

(event `TicketsPrinted`
  (`KismetSystemLibrary.PrintString` "display text to pickup tickets as collectible item"))

(event `EnhancedInput|/Game/ThirdPerson/Input/Actions/IA_Interact`
  (params (ActionValue :type Boolean) (ElapsedSeconds :type "Float (double-precision)") (TriggeredSeconds :type "Float (double-precision)") (InputAction :type "InputAction Object Reference" :default "/Game/ThirdPerson/Input/Actions/IA_Interact.IA_Interact"))
  (bind _ball (`self.Ball`))
  (bind _ball_2 (`self.Ball`))
  (bind _playerref (`self.PlayerRef`))
  (bind _audio (`self.Audio`))
  (bind _returnvalue (`self.K2_GetActorLocation` _playerref))
  (:`Started`
    (if (`/Game/Blueprints/MyBlueprints/BP_ElectricalBox.bIsPowerOn` (`self.BP_PowerBox`))
      (if (`PrimitiveComponent.IsOverlappingActor` (`self.InteractArea`) (`self.PlayerRef`))
        ;[1 1 1] show machine is interactible
        (if (`self.bIsCompleted`)
          ;[0.4202 1 0] if tickets printed, allow e to be the last interaction to take the tickets.
          (if (`self.bTicketsPrinted`)
            (`/Game/ThirdPerson/Blueprints/BP_ThirdPersonCharacter.UpdatePCount` _playerref)
            (`GameplayStatics.PlaySoundAtLocation` "/Game/Audio/note.note" _returnvalue (struct) 1.0 1.0 0.0 null null null null)
            (`GameplayStatics.SpawnEmitterAtLocation` "/Game/VFX/Cascade/P_Impact_Shield.P_Impact_Shield" _returnvalue)
            (`self.K2_DestroyActor` (`self.BP_TicketsRef`))
            (set `self.bTicketsPrinted` false)
            (`/Game/ThirdPerson/Blueprints/BP_ThirdPersonCharacter.UpdateObjective` (`self.PlayerRef`) "NewEnumerator12"))
          (else
            (if (not (`AudioComponent.IsPlaying` _audio))
              (`AudioComponent.Play` _audio 0.0))
            (if (not (`self.bRolledBall`))
              (`SceneComponent.SetVisibility` (`self.ScoreText`) true false)
              (`SceneComponent.SetVisibility` (`self.Arrow`) true false)
              (`SceneComponent.SetVisibility` (`self.Ball`) true false)
              (`SceneComponent.SetVisibility` (`self.InteractText`) false false)
              (if (`self.bUpdatingHorizontalAngle`) :!label _label
                (if (`self.bUpdatingPower`)
                  ;[1 1 1] throw ball
                  (`KismetSystemLibrary.K2_ClearTimer` null "UpdatePower")
                  (`SceneComponent.SetVisibility` (`self.Widget_SkeeballPower`) false false)
                  (`SceneComponent.SetVisibility` (`self.Arrow`) false false)
                  (`PrimitiveComponent.SetSimulatePhysics` (`self.Ball`) true)
                  (`PrimitiveComponent.AddImpulse` _ball (* (`SceneComponent.GetForwardVector` _ball) (`KismetMathLibrary.MapRangeClamped` (`self.CurrentPower`) 0.0 1.0 150.0 350.0)) "None" false)
                  (`PrimitiveComponent.AddTorqueInDegrees` _ball_2 (* (`SceneComponent.GetForwardVector` _ball_2) 1.0) "None" false)
                  (set `self.bRolledBall` true)
                  (else
                    (`KismetSystemLibrary.K2_ClearTimer` null "UpdateHorizontalAngle")
                    (`SceneComponent.SetVisibility` (`self.Widget_HorizontalPosition`) false false)
                    (`SceneComponent.SetVisibility` (`self.Widget_SkeeballPower`) true false)
                    (set `self.bUpdatingPower` true)
                    (`KismetSystemLibrary.K2_SetTimer` null "UpdatePower" 0.016 true)))
                (else
                  (`SceneComponent.SetVisibility` (`self.Widget_HorizontalPosition`) true false)
                  (`SceneComponent.SetVisibility` (`self.Arrow`) true false)
                  (set `self.bUpdatingHorizontalAngle` true)
                  (`KismetSystemLibrary.K2_SetTimer` null "UpdateHorizontalAngle" 0.016 true))))))))))

(event `Key|F`
  (params (Key :type "Key Structure"))
  ;[1 0.4059 0 1 146] DEBUG ONLY
)

(event `self.RolledDownArea.OnComponentBeginOverlap`
  (params (OverlappedComponent :type "PrimitiveComponent Object Reference") (OtherActor :type "Actor Object Reference") (OtherComp :type "PrimitiveComponent Object Reference") (OtherBodyIndex :type Integer) (bFromSweep :type Boolean) (SweepResult :type "HitResult Structure (by ref)"))
  (if (== OtherComp (`self.Ball`))
    (`KismetSystemLibrary.PrintString` "ball entered rolled down area. resetting transform")
    (if (`self.bIsCompleted`) :!label _label_2
      (`self.ClearTimers`)
      (else
        (`self.ResetBall`)
        ;[1 1 1] need a double check to prevent timers from restarting after game ends.
        ; Check if Game Over updates IsCompleted = True after previously selecting isCompleted -> false branch!
        (`self.CheckIfGameOver`)
        (if (not (`self.bIsCompleted`))
          (goto _label))))))

(event `EnhancedInput|/Game/ThirdPerson/Input/Actions/IA_Reset`
  (params (ActionValue :type Boolean) (ElapsedSeconds :type "Float (double-precision)") (TriggeredSeconds :type "Float (double-precision)") (InputAction :type "InputAction Object Reference" :default "/Game/ThirdPerson/Input/Actions/IA_Reset.IA_Reset"))
  (:`Started`
    (if (`/Game/Blueprints/MyBlueprints/BP_ElectricalBox.bIsPowerOn` (`self.BP_PowerBox`))
      (goto _label_2))))

(event `self.100PointsL.OnComponentBeginOverlap`
  (params (OverlappedComponent :type "PrimitiveComponent Object Reference") (OtherActor :type "Actor Object Reference") (OtherComp :type "PrimitiveComponent Object Reference") (OtherBodyIndex :type Integer) (bFromSweep :type Boolean) (SweepResult :type "HitResult Structure (by ref)"))
  ;[1 0 0.5863] Add points based on overlapped area
  (if (== OtherComp (`self.Ball`))
    (set `self.CurrentScore` (+ (`self.CurrentScore`) 100))
    ;[1 0.7445 0] update score text
    (`TextRenderComponent.K2_SetText` (`self.ScoreText`) (`KismetTextLibrary.Conv_IntToText` (`self.CurrentScore`)) :!label _label_3)
    (`GameplayStatics.PlaySoundAtLocation` "/Game/Audio/Video-Game-Unlock-Sound-A1-8bit-www_fesliyanstudios_com.Video-Game-Unlock-Sound-A1-8bit-www_fesliyanstudios_com" (`SceneComponent.K2_GetComponentLocation` (`self.ScoreText`)) (struct) 1.0 1.0 0.0 null null null null)
    (`self.ResetBall`)))

(event `self.100PointsR.OnComponentBeginOverlap`
  (params (OverlappedComponent :type "PrimitiveComponent Object Reference") (OtherActor :type "Actor Object Reference") (OtherComp :type "PrimitiveComponent Object Reference") (OtherBodyIndex :type Integer) (bFromSweep :type Boolean) (SweepResult :type "HitResult Structure (by ref)"))
  ;[1 0 0.5863] Add points based on overlapped area
  (if (== OtherComp (`self.Ball`))
    (set `self.CurrentScore` (+ (`self.CurrentScore`) 100))
    (goto _label_3)))

(event `self.50Points.OnComponentBeginOverlap`
  (params (OverlappedComponent :type "PrimitiveComponent Object Reference") (OtherActor :type "Actor Object Reference") (OtherComp :type "PrimitiveComponent Object Reference") (OtherBodyIndex :type Integer) (bFromSweep :type Boolean) (SweepResult :type "HitResult Structure (by ref)"))
  ;[1 0 0.5863] Add points based on overlapped area
  (if (== OtherComp (`self.Ball`))
    (set `self.CurrentScore` (+ (`self.CurrentScore`) 50))
    (goto _label_3)))

(event `self.40Points.OnComponentBeginOverlap`
  (params (OverlappedComponent :type "PrimitiveComponent Object Reference") (OtherActor :type "Actor Object Reference") (OtherComp :type "PrimitiveComponent Object Reference") (OtherBodyIndex :type Integer) (bFromSweep :type Boolean) (SweepResult :type "HitResult Structure (by ref)"))
  ;[1 0 0.5863] Add points based on overlapped area
  (if (== OtherComp (`self.Ball`))
    (set `self.CurrentScore` (+ (`self.CurrentScore`) 40))
    (goto _label_3)))

(event `self.30Points.OnComponentBeginOverlap`
  (params (OverlappedComponent :type "PrimitiveComponent Object Reference") (OtherActor :type "Actor Object Reference") (OtherComp :type "PrimitiveComponent Object Reference") (OtherBodyIndex :type Integer) (bFromSweep :type Boolean) (SweepResult :type "HitResult Structure (by ref)"))
  ;[1 0 0.5863] Add points based on overlapped area
  (if (== OtherComp (`self.Ball`))
    (set `self.CurrentScore` (+ (`self.CurrentScore`) 30))
    (goto _label_3)))

(event `self.20Points.OnComponentBeginOverlap`
  (params (OverlappedComponent :type "PrimitiveComponent Object Reference") (OtherActor :type "Actor Object Reference") (OtherComp :type "PrimitiveComponent Object Reference") (OtherBodyIndex :type Integer) (bFromSweep :type Boolean) (SweepResult :type "HitResult Structure (by ref)"))
  ;[1 0 0.5863] Add points based on overlapped area
  (if (== OtherComp (`self.Ball`))
    (set `self.CurrentScore` (+ (`self.CurrentScore`) 20))
    (goto _label_3)))

(event `self.10Points.OnComponentBeginOverlap`
  (params (OverlappedComponent :type "PrimitiveComponent Object Reference") (OtherActor :type "Actor Object Reference") (OtherComp :type "PrimitiveComponent Object Reference") (OtherBodyIndex :type Integer) (bFromSweep :type Boolean) (SweepResult :type "HitResult Structure (by ref)"))
  ;[1 0 0.5863] Add points based on overlapped area
  (if (== OtherComp (`self.Ball`))
    (set `self.CurrentScore` (+ (`self.CurrentScore`) 10))
    (goto _label_3)))

(fn `CheckIfDonePrintingTickets`
  (if (`/Game/Blueprints/MyBlueprints/BP_Tickets.bDonePrinting` (`self.BP_TicketsRef`))
    (`KismetSystemLibrary.K2_ClearTimer` null "CheckIfDonePrintingTickets")
    (set `self.bTicketsPrinted` true)
    (`self.TicketsPrinted`)))

(fn `CheckIfGameOver`
  (if (<= (`self.NumBallsShot`) (`self.MaxNumBalls`))
    _
    (elif (>= (`self.CurrentScore`) 300)
      (`KismetSystemLibrary.PrintString` "BP_SkeeballMachine: points exceed 300. game over" true true (struct :`R` 0.000905 :`G` 1.0 :`A` 1.0) 4.0)
      (set `self.bIsCompleted` true)
      (`self.ClearTimers`)
      (`AudioComponent.Stop` (`self.Audio`))
      (`SceneComponent.SetVisibility` (`self.InteractText`) false false)
      (`SceneComponent.SetVisibility` (`self.Widget_SkeeballPower`) false false)
      (`SceneComponent.SetVisibility` (`self.Widget_HorizontalPosition`) false false)
      (`SceneComponent.SetVisibility` (`self.Arrow`) false false)
      (`SceneComponent.SetVisibility` (`self.Ball`) false false)
      (`self.CamExitSkeeball`)
      (bind _returnvalue (`|SpawnActorFromClass` "/Game/Blueprints/MyBlueprints/BP_Tickets.BP_Tickets_C" (`SceneComponent.K2_GetComponentToWorld` (`self.TicketSpawnLocation`)) "Undefined" "MultiplyWithRoot" null null))
      (bind _output_get (set `self.BP_TicketsRef` _returnvalue))
      (set `/Game/Blueprints/MyBlueprints/BP_Tickets.bDonePrinting` false _output_get)
      (`/Game/Blueprints/MyBlueprints/BP_Tickets.SpitOutTickets` _output_get)
      (`KismetSystemLibrary.K2_SetTimer` null "CheckIfDonePrintingTickets" 0.1 true)
      (else
        (`KismetSystemLibrary.PrintString` "BP_SkeeballMachine: resetting game" true true (struct :`R` 1.0 :`B` 0.026111 :`A` 1.0) 4.0)))))

(fn `ClearTimers`
  (`KismetSystemLibrary.K2_ClearTimer` null "UpdateHorizontalAngle")
  (`KismetSystemLibrary.K2_ClearTimer` null "UpdatePower"))

(fn `ResetBall`
  (bind _ball (`self.Ball`))
  (bind _ball7 (`self.Ball7`))
  (bind _ball6 (`self.Ball6`))
  (bind _ball2 (`self.Ball2`))
  (bind _ball3 (`self.Ball3`))
  (bind _ball4 (`self.Ball4`))
  (bind _ball5 (`self.Ball5`))
  (`self.ClearTimers`)
  (if (not (`self.bIsCompleted`))
    (`/Engine/EditorBlueprintResources/StandardMacros.IncrementInt` (`self.NumBallsShot`)
      (:`  `
        (`/Engine/EditorBlueprintResources/StandardMacros.IsValid` _ball2
          (:`Is Valid`
            (`SceneComponent.SetVisibility` _ball2 false false))
          (:`Is Not Valid`
            (`/Engine/EditorBlueprintResources/StandardMacros.IsValid` _ball3
              (:`Is Valid`
                (`SceneComponent.SetVisibility` _ball3 false false))
              (:`Is Not Valid`
                (`/Engine/EditorBlueprintResources/StandardMacros.IsValid` _ball4
                  (:`Is Valid`
                    (`SceneComponent.SetVisibility` _ball4 false false))
                  (:`Is Not Valid`
                    (`/Engine/EditorBlueprintResources/StandardMacros.IsValid` _ball5
                      (:`Is Valid`
                        (`SceneComponent.SetVisibility` _ball5 false false))
                      (:`Is Not Valid`
                        (`/Engine/EditorBlueprintResources/StandardMacros.IsValid` _ball6
                          (:`Is Valid`
                            (`SceneComponent.SetVisibility` _ball6 false false))
                          (:`Is Not Valid`
                            (`/Engine/EditorBlueprintResources/StandardMacros.IsValid` _ball7
                              (:`Is Valid`
                                (`SceneComponent.SetVisibility` _ball7 false false)))))))))))))
        (`PrimitiveComponent.SetSimulatePhysics` _ball false)
        (`SceneComponent.K2_SetWorldTransform` _ball (`self.BallStartTransform`) false false)
        (set `self.bUpdatingHorizontalAngle` false)
        (set `self.bUpdatingPower` false)
        (`self.UpdateScore`)
        (set `self.bRolledBall` false)))))

(fn `UpdateHorizontalAngle`
  (bind (_ballstarttransform_location _ballstarttransform_rotation) (`KismetMathLibrary.BreakTransform` (`self.BallStartTransform`)))
  (bind _worldhorizontalangle (`self.WorldHorizontalAngle`))
  (bind _yaw (.yaw _ballstarttransform_rotation))
  (if (`self.bRight`)
    (if (< (`self.CurrentHorizontalAngle`) (`self.MaxHorizontalAngle`))
      (set `self.CurrentHorizontalAngle` (+ (`self.CurrentHorizontalAngle`) (`self.UpdateAmount`)))
      (`SceneComponent.K2_SetWorldRotation` (`self.Ball`) (`KismetMathLibrary.MakeRotator` (.roll _ballstarttransform_rotation) (.pitch _ballstarttransform_rotation) (`KismetMathLibrary.MapRangeClamped` (`self.CurrentHorizontalAngle`) 0.0 1.0 (- _yaw _worldhorizontalangle) (+ _yaw _worldhorizontalangle))) false false :!label _label)
      (else
        (set `self.bRight` false)))
    (elif (> (`self.CurrentHorizontalAngle`) (`self.MinHorizontalAngle`))
      (set `self.CurrentHorizontalAngle` (- (`self.CurrentHorizontalAngle`) (`self.UpdateAmount`)))
      (goto _label)
      (else
        (set `self.bRight` true)))))

(fn `UpdatePower`
  (bind _arrow (`self.Arrow`))
  (bind (_relativescale3d_x _relativescale3d_y _relativescale3d_z) (`KismetMathLibrary.BreakVector` (`SceneComponent.RelativeScale3D` _arrow)))
  (if (`self.bRight`)
    (if (< (`self.CurrentPower`) (`self.MaxPower`))
      (set `self.CurrentPower` (+ (`self.CurrentPower`) (`self.UpdateAmount`)))
      (`SceneComponent.SetRelativeScale3D` _arrow (`KismetMathLibrary.MakeVector` (`KismetMathLibrary.MapRangeClamped` (`self.CurrentPower`) 0.0 1.0 7.0 22.0) _relativescale3d_y _relativescale3d_z) :!label _label)
      (else
        (set `self.bRight` false)))
    (elif (> (`self.CurrentPower`) (`self.MinPower`))
      (set `self.CurrentPower` (- (`self.CurrentPower`) (`self.UpdateAmount`)))
      (goto _label)
      (else
        (set `self.bRight` true)))))

(fn `UpdateScore`
  (bind _returnvalue (`KismetTextLibrary.Conv_TextToString` (`KismetTextLibrary.Conv_IntToText` (`self.CurrentScore`))))
  (bind _returnvalue_2 (`KismetStringLibrary.Len` _returnvalue))
  (if (== _returnvalue_2 1)
    ;[1 1 1] adds leading zeroes
    (`TextRenderComponent.K2_SetText` (`self.ScoreText`) (`KismetTextLibrary.Conv_StringToText` (`KismetStringLibrary.Concat_StrStr` "00" _returnvalue)))
    (elif (== _returnvalue_2 2)
      (`TextRenderComponent.K2_SetText` (`self.ScoreText`) (`KismetTextLibrary.Conv_StringToText` (`KismetStringLibrary.Concat_StrStr` "0" _returnvalue)))
      (elif (== _returnvalue_2 3)
        (`TextRenderComponent.K2_SetText` (`self.ScoreText`) (`KismetTextLibrary.Conv_IntToText` (`self.CurrentScore`)))))))

(fn `UserConstructionScript`)