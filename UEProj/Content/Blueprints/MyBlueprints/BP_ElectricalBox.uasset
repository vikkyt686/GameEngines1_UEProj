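; Electrical power box that the player toggles on and off with an equipped wrench, driving objective and narration progress.
; Overlapping the interact area shows a prompt, or sends the player to find a wrench.
; Interacting toggles power if an objective update succeeds (or DebugPower is set), changing the light and sound and calling CallPowerOn.
; A looping timer polls the startup sound, then swaps in the running loop.
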(event `self.ReceiveBeginPlay`
  (bind _bispoweron (`self.bIsPowerOn`))
  (bind _audio (`self.Audio`))
  (bind _asbp_third_person_character (cast `/Game/ThirdPerson/Blueprints/BP_ThirdPersonCharacter` (`GameplayStatics.GetPlayerCharacter` 0))
    (:`then`
      (set `self.The Player` _asbp_third_person_character))
    (:`CastFailed`
      (bind _returnvalue (`GameplayStatics.GetActorOfClass` "/Game/ThirdPerson/Blueprints/BP_ThirdPersonCharacter.BP_ThirdPersonCharacter_C"))
      (set `self.The Player` _returnvalue)))
  (`self.EnableInput` (`GameplayStatics.GetPlayerController` 0))
  (if _bispoweron
    (`AudioComponent.SetSound` _audio (select `bool` _bispoweron :`true` "/Game/Audio/Light-Turning-On-A1_Loop-www_fesliyanstudios_com.Light-Turning-On-A1_Loop-www_fesliyanstudios_com" :!type "SoundBase Object Reference"))
    (`AudioComponent.Play` _audio 0.0)))

(event `self.InteractArea.OnComponentBeginOverlap`
  (params (OverlappedComponent :type "PrimitiveComponent Object Reference") (OtherActor :type "Actor Object Reference") (OtherComp :type "PrimitiveComponent Object Reference") (OtherBodyIndex :type Integer) (bFromSweep :type Boolean) (SweepResult :type "HitResult Structure (by ref)"))
  (bind _the_player (`self.The Player`))
  (bind _asbp_third_person_character (cast `/Game/ThirdPerson/Blueprints/BP_ThirdPersonCharacter` OtherActor))
  (if (`/Game/ThirdPerson/Blueprints/BP_ThirdPersonCharacter.bEquippedWrench` _asbp_third_person_character)
    (`SceneComponent.SetVisibility` (`self.InteractText`) true false)
    (`/Game/ThirdPerson/Blueprints/BP_ThirdPersonCharacter.Narrate` (`self.The Player`) "/Game/Audio/Narration/09_now_lets_see_if_we_can_turn_the_power_off_01.09_now_lets_see_if_we_can_turn_the_power_off_01" 9)
    (if (< (`self.NumDisplayedMsgs`) 2)
      (bind _output_get (set `/Game/ThirdPerson/Blueprints/BP_ThirdPersonCharacter.Message Text` "Interact with powerbox?" _asbp_third_person_character))
      (set `self.MyMessage` _output_get)
      (`/Engine/EditorBlueprintResources/StandardMacros.IncrementInt` (`self.NumDisplayedMsgs`)
        (:`  `
          (`/Game/ThirdPerson/Blueprints/BP_ThirdPersonCharacter.DisplayMessage` (`self.The Player`) (`self.MyMessage`) (`self.Display Time`)))))
    (else
      (`/Game/ThirdPerson/Blueprints/BP_ThirdPersonCharacter.UpdateObjective` _the_player "NewEnumerator2")
      (`/Game/ThirdPerson/Blueprints/BP_ThirdPersonCharacter.Narrate` _the_player "/Game/Audio/Narration/08_looks_like_ill_need_a_wrench_01.08_looks_like_ill_need_a_wrench_01" 8))))

(event `self.InteractArea.OnComponentEndOverlap`
  (params (OverlappedComponent :type "PrimitiveComponent Object Reference") (OtherActor :type "Actor Object Reference") (OtherComp :type "PrimitiveComponent Object Reference") (OtherBodyIndex :type Integer))
  (`SceneComponent.SetVisibility` (`self.InteractText`) false false))

(event `EnhancedInput|/Game/ThirdPerson/Input/Actions/IA_Interact`
  (params (ActionValue :type Boolean) (ElapsedSeconds :type "Float (double-precision)") (TriggeredSeconds :type "Float (double-precision)") (InputAction :type "InputAction Object Reference" :default "/Game/ThirdPerson/Input/Actions/IA_Interact.IA_Interact"))
  (bind _the_player (`self.The Player`))
  (bind _bispoweron (`self.bIsPowerOn`))
  (bind _audio (`self.Audio`))
  (:`Started`
    (if (`self.DebugPower`)
      (set `self.bIsPowerOn` (not _bispoweron) :!label _label)
      (`LightComponent.SetLightColor` (`self.PowerLight`) (select `bool` _bispoweron :`false` (`self.Col_LightOff`) :`true` (`self.Col_LightOn`)) true)
      (`AudioComponent.SetSound` _audio (select `bool` _bispoweron :`false` "/Game/Audio/Light-Turning-On-A1_End-www_fesliyanstudios_com.Light-Turning-On-A1_End-www_fesliyanstudios_com" :`true` "/Game/Audio/Light-Turning-On-A1-www_fesliyanstudios_com.Light-Turning-On-A1-www_fesliyanstudios_com" :!type "SoundBase Object Reference"))
      (`AudioComponent.Play` _audio 0.0)
      (`self.PowerOn`)
      (if _bispoweron
        (`KismetSystemLibrary.K2_SetTimer` null "CheckIsAudioPlaying" 0.05 true))
      (elif (`PrimitiveComponent.IsOverlappingActor` (`self.InteractArea`) _the_player)
        (if (`/Game/ThirdPerson/Blueprints/BP_ThirdPersonCharacter.bEquippedWrench` _the_player)
          (bind _bupdatedobjective (`/Game/ThirdPerson/Blueprints/BP_ThirdPersonCharacter.UpdateObjective` _the_player "NewEnumerator5"))
          (`/Game/ThirdPerson/Blueprints/BP_ThirdPersonCharacter.Narrate` (`self.The Player`) "/Game/Audio/Narration/10_i_hope_that_never_happens_to_me_again_01_Cue.10_i_hope_that_never_happens_to_me_again_01_Cue" 10)
          (if _bupdatedobjective
            (goto _label)
            (else
              (bind _bupdatedobjective_2 (`/Game/ThirdPerson/Blueprints/BP_ThirdPersonCharacter.UpdateObjective` _the_player "NewEnumerator11"))
              (if _bupdatedobjective_2
                (`/Game/ThirdPerson/Blueprints/BP_ThirdPersonCharacter.Narrate` (`self.The Player`) "/Game/Audio/Narration/15_sometimes_i_wish_i_could_be_a_kid_again_01.15_sometimes_i_wish_i_could_be_a_kid_again_01" 15)
                (goto _label)))))))))

(fn `CheckIsAudioPlaying`
  (bind _audio (`self.Audio`))
  (if (not (`AudioComponent.IsPlaying` (`self.Audio`)))
    (`AudioComponent.SetSound` _audio "/Game/Audio/Light-Turning-On-A1_Loop-www_fesliyanstudios_com.Light-Turning-On-A1_Loop-www_fesliyanstudios_com")
    (`AudioComponent.Play` _audio 0.0)
    (`KismetSystemLibrary.K2_ClearTimer` null "CheckIsAudioPlaying")))

(fn `UserConstructionScript`)