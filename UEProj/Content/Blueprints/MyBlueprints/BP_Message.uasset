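; BP_Message is a world trigger that updates the player's objective on overlap, whether on foot or driving the sports car.
; An accepted update animates the character or vehicle HUD, optionally plays narration, and can destroy the actor after a short delay.
; The car path resolves the driver through the pawn's character reference.
; A separate SetAndDisplayMessage function shows message text with a sound, tracked by a Displayed flag, but is not called here.
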(event `self.ReceiveBeginPlay`
  (bind _asbp_third_person_character (cast `/Game/ThirdPerson/Blueprints/BP_ThirdPersonCharacter` (`GameplayStatics.GetPlayerCharacter` 0)))
  (set `self.The Player` _asbp_third_person_character))

(event `self.MessageTrigger.OnComponentBeginOverlap`
  (params (OverlappedComponent :type "PrimitiveComponent Object Reference") (OtherActor :type "Actor Object Reference") (OtherComp :type "PrimitiveComponent Object Reference") (OtherBodyIndex :type Integer) (bFromSweep :type Boolean) (SweepResult :type "HitResult Structure (by ref)"))
  (bind _currobjective (`self.CurrObjective`))
  (if (not (`self.bPendingDestroy`))
    (bind _asbp_third_person_character (cast `/Game/ThirdPerson/Blueprints/BP_ThirdPersonCharacter` OtherActor)
      (:`then`
        (bind _output_get (set `self.The Player` _asbp_third_person_character))
        (bind _bupdatedobjective (`/Game/ThirdPerson/Blueprints/BP_ThirdPersonCharacter.UpdateObjective` _output_get (`self.CurrObjective`)))
        (if _bupdatedobjective
          (`/Game/InterfaceWidgets/HUDWidget.AnimateNewObjective` (`/Game/ThirdPerson/Blueprints/BP_ThirdPersonCharacter.My HUD` (`self.The Player`)) :!label _label)
          (if (`self.bNarrate`) :!label _label_2
            (`/Game/ThirdPerson/Blueprints/BP_ThirdPersonCharacter.Narrate` (`self.The Player`) (`self.NarrationAudio`)))
          (if (`self.bDestroyOnceRead`)
            (set `self.bPendingDestroy` true)
            (`KismetSystemLibrary.Delay` 3.0)
            (`self.K2_DestroyActor`))))
      (:`CastFailed`
        (bind _assports_car_pawn (cast `/Game/VehicleTemplate/Blueprints/SportsCar/SportsCar_Pawn` OtherActor))
        (bind _output_get_2 (set `self.The Player` (`/Game/VehicleTemplate/Blueprints/SportsCar/SportsCar_Pawn.TPCharRef` _assports_car_pawn)))
        (bind _bupdatedobjective_2 (`/Game/ThirdPerson/Blueprints/BP_ThirdPersonCharacter.UpdateObjective` _output_get_2 _currobjective))
        (if _bupdatedobjective_2
          (bind _asvehicle_player_controller (cast `/Game/VehicleTemplate/Blueprints/VehiclePlayerController` (`GameplayStatics.GetPlayerController` 0))
            (:`then`
              (bind _vehiclehud (`/Game/VehicleTemplate/Blueprints/VehiclePlayerController.VehicleHud` _asvehicle_player_controller))
              (set `/Game/ThirdPerson/Blueprints/BP_ThirdPersonCharacter.CurrObjective` _currobjective (`/Game/VehicleTemplate/Blueprints/VehicleUI.My Player` _vehiclehud))
              (`/Game/VehicleTemplate/Blueprints/VehicleUI.AnimateNewObjective` _vehiclehud)
              (goto _label_2))
            (:`CastFailed`
              (goto _label))))))))

(fn `Set and Display Message`
  (bind _bdisplayed (`self.bDisplayed`))
  (if (`self.bDisplayOnce`)
    (if (not _bdisplayed)
      (`/Game/ThirdPerson/Blueprints/BP_ThirdPersonCharacter.DisplayMessage` (`self.The Player`) (`self.MyMessage`) (`self.Display Time`) :!label _label)
      (`GameplayStatics.PlaySoundAtLocation` "/Game/Audio/Rollover.Rollover" (`self.K2_GetActorLocation`) (struct) 1.0 1.0 0.0 null null null null :!label _label_2)
      (set `self.bDisplayed` true))
    (elif _bdisplayed
      (goto _label_2)
      (else
        (goto _label)))))

(fn `UserConstructionScript`)