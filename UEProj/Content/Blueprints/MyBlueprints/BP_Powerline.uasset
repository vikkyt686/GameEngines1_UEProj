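; Powerline actor that places a pole mesh at every point of its spline from the construction script.
; Each pole takes the point's transform with a global rotation offset and doubled scale.
; Its LAttach and RAttach socket transforms are stored in arrays, in world and actor space respectively.
; Spline-mesh wires between those sockets, an instanced-mesh variant and test lights are present but disconnected, so no wires are built.
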(fn `PlacePowerlineMeshes`
  (bind _spline (`self.Spline`))
  (for _index (range (`SplineComponent.GetNumberOfSplinePoints` _spline))
    (bind _returnvalue (`AddComponent|NODE_AddStaticMeshComponent-0` :`RelativeTransform` (`KismetMathLibrary.MakeTransform` (.location (`SplineComponent.GetTransformAtSplinePoint` _spline _index "Local" false)) (`KismetMathLibrary.ComposeRotators` (.rotation (`SplineComponent.GetTransformAtSplinePoint` _spline _index "Local" false)) (`self.GlobalRotationOffset`)) (* (.scale (`SplineComponent.GetTransformAtSplinePoint` _spline _index "Local" false)) 2.0))))
    (`StaticMeshComponent.SetStaticMesh` _returnvalue "/Game/Meshes/SM_PowerLine_PROXY_01.SM_PowerLine_PROXY_01")
    (`KismetArrayLibrary.Array_Add` (`self.LAttachTransforms`) (`SceneComponent.GetSocketTransform` _returnvalue "LAttach" "RTS_World"))
    (`KismetArrayLibrary.Array_Add` (`self.RAttachTransforms`) (`SceneComponent.GetSocketTransform` _returnvalue "RAttach" "RTS_Actor"))))

(fn `UserConstructionScript`
  (`self.PlacePowerlineMeshes`))