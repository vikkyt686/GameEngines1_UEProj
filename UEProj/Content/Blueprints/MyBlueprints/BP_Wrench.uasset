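; BP_Wrench is a collectible wrench that the player picks up by walking into it.
; When its CollectionTrigger is overlapped and it is not hidden, it flags the wrench as equipped on the player and calls CollectiblePickedUp.
; It then has the player equip the wrench, advances the objective with a sound effect, and plays the HUD's collected-item animation.
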(event `self.CollectionTrigger.OnComponentBeginOverlap`
  (params (OverlappedComponent :type "PrimitiveComponent Object Reference") (OtherActor :type "Actor Object Reference") (OtherComp :type "PrimitiveComponent Object Reference") (OtherBodyIndex :type Integer) (bFromSweep :type Boolean) (SweepResult :type "HitResult Structure (by ref)"))
  (bind _the_player (`self.The Player`))
  (bind _my_hud (`/Game/ThirdPerson/Blueprints/BP_ThirdPersonCharacter.My HUD` _the_player))
  (if (not (`self.bHidden`))
    (set `/Game/ThirdPerson/Blueprints/BP_ThirdPersonCharacter.bEquippedWrench` true _the_player)
    (`self.CollectiblePickedUp`)
    (`/Game/ThirdPerson/Blueprints/BP_ThirdPersonCharacter.EquipWrench` _the_player)
    (`/Game/ThirdPerson/Blueprints/BP_ThirdPersonCharacter.UpdateObjective` _the_player "NewEnumerator4" true)
    (`UserWidget.PlayAnimation` _my_hud (`/Game/InterfaceWidgets/HUDWidget.CollectedItem` _my_hud) 0.0 1 "Forward" 1.0 false)))

(fn `UserConstructionScript`
  (`parent.UserConstructionScript`))