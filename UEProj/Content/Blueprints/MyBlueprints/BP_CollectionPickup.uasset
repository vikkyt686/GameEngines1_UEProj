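; BP_CollectionPickup is a collectible that the third-person player character picks up by overlapping its trigger.
; BeginPlay caches the player character, falling back to an actor-of-class search if the cast fails.
; On overlap, CollectiblePickedUp updates the player's pickup count, plays a sound and particle effect, then destroys the actor.
; A timeline for bobbing and spinning the mesh exists but is never run.
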(event `self.ReceiveBeginPlay`
  (bind _asbp_third_person_character (cast `/Game/ThirdPerson/Blueprints/BP_ThirdPersonCharacter` (`GameplayStatics.GetPlayerCharacter` 0))
    (:`then`
      (set `self.The Player` _asbp_third_person_character))
    (:`CastFailed`
      (bind _returnvalue (`GameplayStatics.GetActorOfClass` "/Game/ThirdPerson/Blueprints/BP_ThirdPersonCharacter.BP_ThirdPersonCharacter_C"))
      (set `self.The Player` _returnvalue))))

(event `self.CollectionTrigger.OnComponentBeginOverlap`
  (params (OverlappedComponent :type "PrimitiveComponent Object Reference") (OtherActor :type "Actor Object Reference") (OtherComp :type "PrimitiveComponent Object Reference") (OtherBodyIndex :type Integer) (bFromSweep :type Boolean) (SweepResult :type "HitResult Structure (by ref)"))
  (cast `/Game/ThirdPerson/Blueprints/BP_ThirdPersonCharacter` OtherActor)
  (`self.CollectiblePickedUp`))

(fn `CollectiblePickedUp`
  (bind _returnvalue (`self.K2_GetActorLocation`))
  (`/Game/ThirdPerson/Blueprints/BP_ThirdPersonCharacter.UpdatePCount` (`self.The Player`))
  (`GameplayStatics.PlaySoundAtLocation` "/Game/Audio/note.note" _returnvalue (struct) 1.0 1.0 0.0 null null null null)
  (`GameplayStatics.SpawnEmitterAtLocation` "/Game/VFX/Cascade/P_Impact_Shield.P_Impact_Shield" _returnvalue)
  (`self.K2_DestroyActor`))

(fn `UserConstructionScript`)